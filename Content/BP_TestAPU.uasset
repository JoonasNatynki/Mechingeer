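; BP_TestAPU is a test APU Blueprint that exposes a set of electrical power functions but is almost entirely stubbed.
; Only the nominal amperage and voltage getters return data, read from its NominalAmperage and NominalVoltage variables.
; IsPoweredOn always returns false, while power consumption, operational readings and the voltage delta are empty.
; Its event graph and construction script do nothing.
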(event EventBeginPlay)

(event Collision|EventActorBeginOverlap
  (params (OtherActor :type Actor%20Object%20Reference)))

(event EventTick
  (params (DeltaSeconds :type Float%20%28single-precision%29)))

(fn ConstructionScript)

(fn ConsumerElectricPower
  (params (DeltaTime :type Float%20%28single-precision%29))
  (return ""))

(fn GetCurrentOperationalAmperage
  (return ""))

(fn GetCurrentOperationalVoltage
  (return ""))

(fn GetCurrentPowerConsumption
  (return ""))

(fn GetNominalAmperage
  (return (Variables|Default|GetNominalAmperage)))

(fn GetNominalVoltage
  (return (Variables|Default|GetNominalVoltage)))

(fn GetVoltageNominalityDelta
  (return ""))

(fn IsPoweredon
  (return false))